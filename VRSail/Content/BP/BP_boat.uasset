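; BP_boat is a player-controlled canoe that moves by physics forces from input axes.
; AddMovementForce pushes the canoe mesh with a scaled, mass-independent force, with Move Forward using the actor's right vector and Move Left its forward vector.
; Move Right ignores its axis value and adds constant controller yaw, while Tick spins the actor at RotationSeed yaw per second.
; A reversed forward-vector force call is left unconnected.
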(event EventBeginPlay)

(event Collision|EventActorBeginOverlap
  (params (OtherActor :type Actor%20Object%20Reference)))

(event EventTick
  (params (DeltaSeconds :type Float%20%28single-precision%29))
  (Transformation|AddActorLocalRotation (* (Math|Rotator|MakeRotator 0.0 0.0 (Variables|Default|GetRotation_seed)) DeltaSeconds) false false))

(event Input|AxisEvents|InputAxisMoveForward
  (params (AxisValue :type Float%20%28single-precision%29))
  (Utilities|AddMovementForce AxisValue (Transformation|GetActorRightVector)))

(event Input|AxisEvents|InputAxisMoveRight
  (params (AxisValue :type Float%20%28single-precision%29))
  (Pawn|Input|AddControllerYawInput 1e+02))

(event Input|AxisEvents|InputAxisMoveLeft
  (params (AxisValue :type Float%20%28single-precision%29))
  (Utilities|AddMovementForce AxisValue (Transformation|GetActorForwardVector)))

(fn ConstructionScript)

(fn NewFunction0)